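; Info point actor with a text label that shows briefly when its Activate event fires.
; Activate opens a gate and unhides the TextRender, then after a 0.2 second delay hides it and closes the gate.
; While the gate is open, Tick rotates the text to face the player pawn.
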(event Custom|Activate
  (bind _textrender (Variables|Default|GetTextRender))
  (bind _textrender_2 (Variables|Default|GetTextRender))
  (Utilities|FlowControl|Sequence
    (:then_0
      (Utilities|FlowControl|Gate true) ; enters at Open
    )
    (:then_1
      (Development|SetHiddeninGame _textrender_2 false false)
      (Utilities|FlowControl|Delay 0.2)
      (Development|SetHiddeninGame _textrender_2 true false)
      (Utilities|FlowControl|Gate true) ; enters at Close
    )))

(event EventBeginPlay)

(event Collision|EventActorBeginOverlap
  (params (OtherActor :type Actor%20Object%20Reference)))

(event EventTick
  (params (DeltaSeconds :type Float%20%28single-precision%29))
  (bind _textrender (Variables|Default|GetTextRender))
  (Utilities|FlowControl|Gate true
    (:Exit
      (Transformation|SetWorldRotation _textrender (Math|Rotator|FindLookatRotation (Transformation|GetWorldLocation _textrender) (Transformation|GetActorLocation (Game|Player|GetPlayerPawn 0))) false false))))

(fn ConstructionScript)