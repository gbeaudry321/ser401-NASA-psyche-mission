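; BP_TestInteractionActor is a test interactable that opens a carousel UI when interacted with.
; Focus toggles custom depth on its Cube for highlighting, and it exposes its Widget through GetInteractionWidgetRef.
; Interact creates and activates WBP_IP_Carousel_Template, switching player 0 to UI-only input with a cursor.
; A RepNotify on InteractToggle drives POI visibility; LookAt returns empty text, and older POI-hiding logic is disconnected.
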(event Collision|EventActorBeginOverlap
  (params (OtherActor :type Actor%20Object%20Reference)))

(event EventInterfaceToggleFocus
  (params (Focus :type Boolean))
  (Rendering|SetRenderCustomDepth (Variables|Default|GetCube) Focus))

(event MouseInput|EventActorOnClicked
  (params (ButtonPressed :type Key%20Structure)))

(event EventInteractwith
  (CallFunction|Interact))

(fn ConstructionScript)

(fn OnRepInteractToggle
  (bind _poi (Variables|Default|GetPOI))
  (if (Variables|Default|GetInteractToggle)
    (Rendering|SetVisibility _poi true false)
    (else
      (Rendering|SetVisibility _poi false false))))

(fn GetInteractionWidgetRef
  (return (Variables|Default|GetWidget)))

(fn Interact
  (params (Interactor :type Actor%20Object%20Reference))
  (bind _returnvalue (Game|GetPlayerController 0))
  (bind _returnvalue_2 (UserInterface|CreateWidget "/Game/UI/InfoPoints/WBP_IP_Carousel_Template.WBP_IP_Carousel_Template_C"))
  (UserInterface|Viewport|AddtoViewport _returnvalue_2 0)
  (Class|CommonActivatableWidget|ActivateWidget _returnvalue_2)
  (Input|SetInputModeUIOnly _returnvalue 0 "DoNotLock" false)
  (Variables|/Script/Engine.PlayerController|SetbShowMouseCursor _returnvalue true)
  (return (Variables|Default|GetVisible)))

(fn Lookat
  (return ""))