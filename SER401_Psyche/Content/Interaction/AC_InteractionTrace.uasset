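; Component that lets the player focus and interact with BP_InteractionArea actors under the camera's view.
; Each Tick runs a Visibility line trace forward from the camera and, when the hit actor changes or the trace misses, updates the area's focus highlight state.
; TryToInteract sends an interface interact message to the focused area's parent actor only when its InteractDuration is not positive; timed interactions have no handling here.
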(event Custom|TryToInteract
  (params (Input :type Boolean))
  (if Input
    (if (Variables|Default|GetIsTracingInteractionArea)
      (bind _output_get (Variables|Default|SetInteract%20Duration_0 (Variables|/Game/Interaction/BP_InteractionArea.BP_InteractionArea_C|GetInteractDuration (Variables|Default|GetFocusedInteractionArea))))
      (if (not (> _output_get 0.0))
        (CallFunction|Interaction (Variables|Default|GetFocusedInteractionArea))))))

(event Custom|Interaction
  (params (InteractionArea :type BP%20Interaction%20Area%20Object%20Reference))
  (Class|BIInteraction|InterfaceInteract(Message) (Actor|GetParentActor InteractionArea)))

(event EventTick
  (params (DeltaSeconds :type Float%20%28single-precision%29))
  (CallFunction|Trace))

(fn Trace
  (bind _returnvalue (Game|GetPlayerCameraManager 0))
  (bind _returnvalue_2 (Transformation|GetActorLocation _returnvalue))
  (bind (_outhit _returnvalue_3) (Collision|LineTraceByChannel _returnvalue_2 (+ _returnvalue_2 (* (Math|Vector|GetForwardVector (Transformation|GetActorRotation _returnvalue)) (Variables|Default|GetLength))) "TraceTypeQuery1" false 0 "None"))
  (if _returnvalue_3
    (if (!= (Variables|Default|GetFocused%20Actor) (.HitActor (Collision|BreakHitResult _outhit)))
      (Variables|Default|SetFocused%20Actor (.HitActor (Collision|BreakHitResult _outhit)))
      (CallFunction|TraceInteractionArea (== (Utilities|GetClass (.HitActor (Collision|BreakHitResult _outhit))) "/Game/Interaction/BP_InteractionArea.BP_InteractionArea_C")))
    (else
      (CallFunction|TraceInteractionArea false))))

(fn TraceInteractionArea
  (params (Trace :type Boolean))
  (if Trace
    (if (Variables|Default|GetIsTracingInteractionArea)
      (Default|ToggleFocused (Variables|Default|GetFocusedInteractionArea) false))
    (bind _asbp_interaction_area (Utilities|Casting|CastToBP_InteractionArea (Variables|Default|GetFocused%20Actor)))
    (bind _output_get (Variables|Default|SetFocusedInteractionArea _asbp_interaction_area))
    (Default|ToggleFocused _output_get true)
    (Variables|Default|SetIsTracingInteractionArea true)
    (elif (Variables|Default|GetIsTracingInteractionArea)
      (Variables|Default|SetIsTracingInteractionArea false)
      (Default|ToggleFocused (Variables|Default|GetFocusedInteractionArea) false)
      (Variables|Default|SetFocused%20Actor 0)
      (Variables|Default|SetFocusedInteractionArea 0))))