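; Base HUD Blueprint that sets game-only input and displays a probe IP head widget on BeginPlay.
; The widget joins a probe IP widget list, whose entries are all added to the viewport.
; Toggle_IP passes the head widget to ToggleWidget, which only stores a valid widget as ActiveWidget without changing visibility.
; Creation of a second, node widget is present but disconnected.
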(event Custom|Toggle_IP
  (CallFunction|ToggleWidget (Variables|Default|GetWB_Probe_Head)))

(event EventBeginPlay
  ;[1 1 1] Focus on Game
  (Input|SetInputModeGameOnly (Game|Player|GetOwningPlayerController) false)
  (bind _returnvalue (UserInterface|CreateWidget "/Game/UI/InfoPoints/IP_Template_Head.IP_Template_Head_C" (Game|Player|GetOwningPlayerController)))
  (bind _output_get (Variables|Default|SetWB_Probe_Head _returnvalue))
  (Utilities|Array|Add (Variables|Default|GetProbe_IP_WidgetList) _output_get)
  (for _array_element (Variables|Default|GetProbe_IP_WidgetList)
    (UserInterface|Viewport|AddtoViewport _array_element 0)))

(fn ConstructionScript)

(fn ToggleWidget
  (params (TargetWidget :type User%20Widget%20Object%20Reference))
  (Utilities|IsValid TargetWidget
    (:Is%20Valid
      (Variables|Default|SetActiveWidget TargetWidget))))